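; Player character Blueprint for a shooter, handling Enhanced Input movement, look, jump, sprint and crouch.
; BeginPlay creates the HUD and passes it the player and the first three BP_Emeny actors found.
; Shooting spawns a bullet with muzzle flash and sound, then decrements ammo; running out pauses the game with a "Win" screen.
; TakeDamage decrements Hp and shows the same game-over widget as "lose" at zero.
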(event Input|EnhancedActionEvents|EnhancedInputActionIA_Move
  (params (ActionValue :type Vector%202D%20Structure) (ElapsedSeconds :type Float%20%28double-precision%29) (TriggeredSeconds :type Float%20%28double-precision%29) (InputAction :type Input%20Action%20Object%20Reference :default "/Game/Input/Actions/IA_Move.IA_Move"))
  ;[0.15 0.15 0.15 0.5] Movement
  (Pawn|Input|AddMovementInput (Transformation|GetActorForwardVector) (.y ActionValue) false)
  (Pawn|Input|AddMovementInput (Transformation|GetActorRightVector) (.x ActionValue) false))

(event Input|EnhancedActionEvents|EnhancedInputActionIA_Shoot
  (params (ActionValue :type Boolean) (ElapsedSeconds :type Float%20%28double-precision%29) (TriggeredSeconds :type Float%20%28double-precision%29) (InputAction :type Input%20Action%20Object%20Reference :default "/Game/Input/Actions/IA_Shoot.IA_Shoot"))
  (bind _returnvalue (Game|GetPlayerController 0))
  (bind _bulletspawnpos (Variables|Default|GetBulletSpawnPos))
  (bind _returnvalue_2 (Transformation|GetWorldTransform _bulletspawnpos))
  (:Started
    (Game|SpawnActorfromClass "/Game/Blueprints/BP_Bullet.BP_Bullet_C" (Math|Transform|MakeTransform (.location _returnvalue_2) (Math|Rotator|MakeRotator (.roll (.rotation _returnvalue_2)) (.pitch (.rotation _returnvalue_2)) (.yaw (.rotation _returnvalue_2))) "1.000000,1.000000,1.000000") "Undefined" "MultiplyWithRoot" 0 0)
    (Niagara|SpawnSystematLocation "/Game/MuzzleFlash/MuzzleFlash/Niagara/NS_MuzzleFlash.NS_MuzzleFlash" (.location _returnvalue_2) (Math|Rotator|MakeRotator (.roll (.rotation _returnvalue_2)) (.pitch (.rotation _returnvalue_2)) (+ (.yaw (.rotation _returnvalue_2)) -9e+01)))
    (Audio|PlaySound2D "/Game/FreeGunSounds/Wav/Rifle/WAV_Rifle_shot01.WAV_Rifle_shot01" 1.0 1.0 0.0 0 0)
    (bind _output_get (Variables|Default|SetBullet (- (Variables|Default|GetBullet) 1)))
    (if (<= _output_get 0)
      (Game|SetGamePaused true)
      (bind _returnvalue_3 (UserInterface|CreateWidget "/Game/Blueprints/WBP_GameOver.WBP_GameOver_C"))
      (Variables|/Script/UMG.TextBlock|SetText (Variables|/Game/Blueprints/WBP_GameOver.WBP_GameOver_C|GetWinLoseText _returnvalue_3) "Win")
      (UserInterface|Viewport|AddtoViewport _returnvalue_3 0)
      (Variables|/Script/Engine.PlayerController|SetbShowMouseCursor _returnvalue true)
      (Input|SetInputModeUIOnly _returnvalue _returnvalue_3 "DoNotLock" false))))

(event Input|EnhancedActionEvents|EnhancedInputActionIA_Jump
  (params (ActionValue :type Boolean) (ElapsedSeconds :type Float%20%28double-precision%29) (TriggeredSeconds :type Float%20%28double-precision%29) (InputAction :type Input%20Action%20Object%20Reference :default "/Game/Input/Actions/IA_Jump.IA_Jump"))
  (Character|Jump))

(event Input|EnhancedActionEvents|EnhancedInputActionIA_Sprint
  (params (ActionValue :type Boolean) (ElapsedSeconds :type Float%20%28double-precision%29) (TriggeredSeconds :type Float%20%28double-precision%29) (InputAction :type Input%20Action%20Object%20Reference :default "/Game/Input/Actions/IA_Sprint.IA_Sprint"))
  (bind _charactermovement (Variables|Character|GetCharacterMovement))
  (:Started
    (Variables|Default|SetisSprinting true)
    (Variables|/Script/Engine.CharacterMovementComponent|SetMaxWalkSpeed _charactermovement (Variables|Default|Getsprintspeed)))
  (:Completed
    (Variables|Default|SetisSprinting false)
    (Variables|/Script/Engine.CharacterMovementComponent|SetMaxWalkSpeed _charactermovement (Variables|Default|Getwalkspeed))))

(event Input|EnhancedActionEvents|EnhancedInputActionIA_Crouch
  (params (ActionValue :type Boolean) (ElapsedSeconds :type Float%20%28double-precision%29) (TriggeredSeconds :type Float%20%28double-precision%29) (InputAction :type Input%20Action%20Object%20Reference :default "/Game/Input/Actions/IA_Crouch.IA_Crouch"))
  (:Started
    (Character|Crouch))
  (:Completed
    (Character|UnCrouch)))

(event Input|EnhancedActionEvents|EnhancedInputActionIA_MouseLook
  (params (ActionValue :type Vector%202D%20Structure) (ElapsedSeconds :type Float%20%28double-precision%29) (TriggeredSeconds :type Float%20%28double-precision%29) (InputAction :type Input%20Action%20Object%20Reference :default "/Game/Input/Actions/IA_MouseLook.IA_MouseLook"))
  (bind _looksensitivity (Variables|Default|GetlookSensitivity))
  ;[0.15 0.15 0.15 0.5] Camera Look
  (Pawn|Input|AddControllerYawInput (* (.x ActionValue) _looksensitivity))
  (Pawn|Input|AddControllerPitchInput (* (.y ActionValue) _looksensitivity)))

(event Collision|EventActorBeginOverlap
  (params (OtherActor :type Actor%20Object%20Reference)))

(event EventTick
  (params (DeltaSeconds :type Float%20%28single-precision%29)))

(event EventBeginPlay
  (bind _returnvalue (Game|GetPlayerController 0))
  (Input|AddMappingContext (PlayerController|LocalPlayerSubsystems|GetEnhancedInputLocalPlayerSubsystem _returnvalue) 0 0 "(bIgnoreAllPressedKeysUntilRelease=True,bForceImmediately=False,bNotifyUserSettings=False)")
  (bind _returnvalue_2 (UserInterface|CreateWidget "/Game/WBP_HUD.WBP_HUD_C" _returnvalue))
  (bind _asbp_player_character (Utilities|Casting|CastToBP_PlayerCharacter (Game|GetPlayerCharacter 0)))
  (Variables|/Game/WBP_HUD.WBP_HUD_C|SetPlayer_Ref _returnvalue_2 _asbp_player_character)
  (UserInterface|Viewport|AddtoViewport _returnvalue_2 0)
  (bind _outactors (Actor|GetAllActorsOfClass "/Game/Blueprints/BP_Emeny.BP_Emeny_C"))
  (Variables|/Game/WBP_HUD.WBP_HUD_C|SetEnemyRef1 _returnvalue_2 (Utilities|Array|Get(acopy) _outactors))
  (Variables|/Game/WBP_HUD.WBP_HUD_C|SetEnemyRef2 _returnvalue_2 (Utilities|Array|Get(acopy) _outactors 1))
  (Variables|/Game/WBP_HUD.WBP_HUD_C|SetEnemyRef3 _returnvalue_2 (Utilities|Array|Get(acopy) _outactors 2)))

(fn ConstructionScript)

(fn TakeDamage
  (bind _returnvalue (Game|GetPlayerController 0))
  (bind _result (Math|Integer|DecrementInt (Variables|Default|Gethp))
    (:%20%20
      (if (<= _result 0)
        (Game|SetGamePaused true)
        (bind _returnvalue_2 (UserInterface|CreateWidget "/Game/Blueprints/WBP_GameOver.WBP_GameOver_C"))
        (Variables|/Script/UMG.TextBlock|SetText (Variables|/Game/Blueprints/WBP_GameOver.WBP_GameOver_C|GetWinLoseText _returnvalue_2) "lose")
        (UserInterface|Viewport|AddtoViewport _returnvalue_2 0)
        (Variables|/Script/Engine.PlayerController|SetbShowMouseCursor _returnvalue true)
        (Input|SetInputModeUIOnly _returnvalue _returnvalue_2 "DoNotLock" false)))))