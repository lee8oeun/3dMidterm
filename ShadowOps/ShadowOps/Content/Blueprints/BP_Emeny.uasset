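; BP_Emeny is a character Blueprint that, despite its name, contains first-person-shooter style player controls and a simple health counter.
; BeginPlay calls AddMappingContext on player 0, and Enhanced Input events drive movement, mouse look, jump, hold-to-sprint and hold-to-crouch.
; Shooting spawns BP_Bullet and a Niagara muzzle flash at BulletSpawnPos with a rifle sound.
; TakeDamage decrements Hp and destroys the actor once it is depleted.
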(event Input|EnhancedActionEvents|EnhancedInputActionIA_Move
  (params (ActionValue :type Vector%202D%20Structure) (ElapsedSeconds :type Float%20%28double-precision%29) (TriggeredSeconds :type Float%20%28double-precision%29) (InputAction :type Input%20Action%20Object%20Reference :default "/Game/Input/Actions/IA_Move.IA_Move"))
  ;[0.15 0.15 0.15 0.5] Movement
  (Pawn|Input|AddMovementInput (Transformation|GetActorForwardVector) (.y ActionValue) false)
  (Pawn|Input|AddMovementInput (Transformation|GetActorRightVector) (.x ActionValue) false))

(event Input|EnhancedActionEvents|EnhancedInputActionIA_Shoot
  (params (ActionValue :type Boolean) (ElapsedSeconds :type Float%20%28double-precision%29) (TriggeredSeconds :type Float%20%28double-precision%29) (InputAction :type Input%20Action%20Object%20Reference :default "/Game/Input/Actions/IA_Shoot.IA_Shoot"))
  (bind _bulletspawnpos (Variables|Default|GetBulletSpawnPos))
  (bind _returnvalue (Transformation|GetWorldTransform _bulletspawnpos))
  (:Started
    (Game|SpawnActorfromClass "/Game/Blueprints/BP_Bullet.BP_Bullet_C" (Math|Transform|MakeTransform (.location _returnvalue) (Math|Rotator|MakeRotator (.roll (.rotation _returnvalue)) (.pitch (.rotation _returnvalue)) (.yaw (.rotation _returnvalue))) "1.000000,1.000000,1.000000") "Undefined" "MultiplyWithRoot" 0 0)
    (Niagara|SpawnSystematLocation "/Game/MuzzleFlash/MuzzleFlash/Niagara/NS_MuzzleFlash.NS_MuzzleFlash" (.location _returnvalue) (Math|Rotator|MakeRotator (.roll (.rotation _returnvalue)) (.pitch (.rotation _returnvalue)) (+ (.yaw (.rotation _returnvalue)) -9e+01)))
    (Audio|PlaySound2D "/Game/FreeGunSounds/Wav/Rifle/WAV_Rifle_shot01.WAV_Rifle_shot01" 1.0 1.0 0.0 0 0)))

(event Input|EnhancedActionEvents|EnhancedInputActionIA_Jump
  (params (ActionValue :type Boolean) (ElapsedSeconds :type Float%20%28double-precision%29) (TriggeredSeconds :type Float%20%28double-precision%29) (InputAction :type Input%20Action%20Object%20Reference :default "/Game/Input/Actions/IA_Jump.IA_Jump"))
  (Character|Jump))

(event Input|EnhancedActionEvents|EnhancedInputActionIA_Sprint
  (params (ActionValue :type Boolean) (ElapsedSeconds :type Float%20%28double-precision%29) (TriggeredSeconds :type Float%20%28double-precision%29) (InputAction :type Input%20Action%20Object%20Reference :default "/Game/Input/Actions/IA_Sprint.IA_Sprint"))
  (bind _charactermovement (Variables|Character|GetCharacterMovement))
  (:Started
    (Variables|Default|SetisSprinting true)
    (Variables|/Script/Engine.CharacterMovementComponent|SetMaxWalkSpeed _charactermovement (Variables|Default|Getsprintspeed)))
  (:Completed
    (Variables|Default|SetisSprinting false)
    (Variables|/Script/Engine.CharacterMovementComponent|SetMaxWalkSpeed _charactermovement (Variables|Default|Getwalkspeed))))

(event Input|EnhancedActionEvents|EnhancedInputActionIA_Crouch
  (params (ActionValue :type Boolean) (ElapsedSeconds :type Float%20%28double-precision%29) (TriggeredSeconds :type Float%20%28double-precision%29) (InputAction :type Input%20Action%20Object%20Reference :default "/Game/Input/Actions/IA_Crouch.IA_Crouch"))
  (:Started
    (Character|Crouch))
  (:Completed
    (Character|UnCrouch)))

(event Input|EnhancedActionEvents|EnhancedInputActionIA_MouseLook
  (params (ActionValue :type Vector%202D%20Structure) (ElapsedSeconds :type Float%20%28double-precision%29) (TriggeredSeconds :type Float%20%28double-precision%29) (InputAction :type Input%20Action%20Object%20Reference :default "/Game/Input/Actions/IA_MouseLook.IA_MouseLook"))
  (bind _looksensitivity (Variables|Default|GetlookSensitivity))
  ;[0.15 0.15 0.15 0.5] Camera Look
  (Pawn|Input|AddControllerYawInput (* (.x ActionValue) _looksensitivity))
  (Pawn|Input|AddControllerPitchInput (* (.y ActionValue) _looksensitivity)))

(event Collision|EventActorBeginOverlap
  (params (OtherActor :type Actor%20Object%20Reference)))

(event EventTick
  (params (DeltaSeconds :type Float%20%28single-precision%29)))

(event EventBeginPlay
  (Input|AddMappingContext (PlayerController|LocalPlayerSubsystems|GetEnhancedInputLocalPlayerSubsystem (Game|GetPlayerController 0)) 0 0 "(bIgnoreAllPressedKeysUntilRelease=True,bForceImmediately=False,bNotifyUserSettings=False)"))

(fn ConstructionScript)

(fn TakeDamage
  (bind _result (Math|Integer|DecrementInt (Variables|Default|Gethp))
    (:%20%20
      (if (<= _result 0)
        (Actor|DestroyActor)))))