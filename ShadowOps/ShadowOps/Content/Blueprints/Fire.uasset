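; Behavior tree task that makes an enemy pawn fire one bullet toward the player.
; It casts the controlled pawn to BP_Emeny, decrements its Ammo without checking the count, and spawns a BP_Bullet at the Muzzle.
; The bullet is rotated toward the PlayerLocation blackboard vector, then the task finishes successfully.
; A failed cast leaves the task without a FinishExecute call.
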(event EventReceiveExecuteAI
  (params (OwnerController :type AI%20Controller%20Object%20Reference) (ControlledPawn :type Pawn%20Object%20Reference))
  (bind _asbp_emeny (Utilities|Casting|CastToBP_Emeny ControlledPawn))
  (bind _result (Math|Integer|DecrementInt (Variables|/Game/Blueprints/BP_Emeny.BP_Emeny_C|Getammo _asbp_emeny))
    (:%20%20
      (Variables|/Game/Blueprints/BP_Emeny.BP_Emeny_C|Setammo _asbp_emeny _result)
      (Game|SpawnActorfromClass "/Game/Blueprints/BP_Bullet.BP_Bullet_C" (Math|Transform|MakeTransform (Transformation|GetWorldLocation (Variables|/Game/Blueprints/BP_Emeny.BP_Emeny_C|GetMuzzle _asbp_emeny)) (Math|Rotator|FindLookatRotation (Transformation|GetWorldLocation (Variables|/Game/Blueprints/BP_Emeny.BP_Emeny_C|GetMuzzle _asbp_emeny)) (Class|BTFunctionLibrary|GetBlackboardValueasVector (Variables|Default|GetPlayerLocation))) "1.000000,1.000000,1.000000") "Undefined" "MultiplyWithRoot" 0 0)
      (AI|BehaviorTree|FinishExecute true))))